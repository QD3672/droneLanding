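; BP_Helipad is a landing pad that drifts horizontally around its starting location at a constant height.
; BeginPlay stores the original location, and ChooseLocation picks a random target offset from it, scaled by Distance.
; Tick eases the actor toward that target with VInterpTo and picks a new one once it is within a small tolerance.
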(event Custom|ChooseLocation
  (bind _returnvalue (Math|Random|RandomUnitVector))
  (bind _distance (Variables|Default|GetDistance))
  (bind _originallocation (Variables|Default|GetOriginalLocation))
  (bind _returnvalue_2 (* _returnvalue _distance))
  (bind _returnvalue_3 (+ _originallocation _returnvalue_2))
  (Variables|Default|SetNewLocation (Math|Vector|MakeVector (.x _returnvalue_3) (.y _returnvalue_3) (.z (Variables|Default|GetOriginalLocation)))))

(event EventBeginPlay
  (Variables|Default|SetOriginalLocation (Transformation|GetActorLocation))
  (CallFunction|ChooseLocation))

(event EventTick
  (params (DeltaSeconds :type Float%20%28single-precision%29))
  (bind _returnvalue (Utilities|Time|GetWorldDeltaSeconds))
  (bind _returnvalue_2 (Transformation|GetActorLocation))
  (bind _newlocation (Variables|Default|GetNewLocation))
  (bind _returnvalue_3 (Math|Interpolation|VInterpTo _returnvalue_2 _newlocation _returnvalue 0.5))
  (Transformation|SetActorLocation (Math|Vector|MakeVector (.x _returnvalue_3) (.y _returnvalue_3) (.z (Variables|Default|GetOriginalLocation))) false false)
  (if (Utilities|Operators|EqualEqual (Transformation|GetActorLocation) (Variables|Default|GetNewLocation) 5e+01)
    (CallFunction|ChooseLocation)))

(fn ConstructionScript)